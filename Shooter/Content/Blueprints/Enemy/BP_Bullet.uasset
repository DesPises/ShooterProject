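; Enemy bullet actor that damages the player on overlap.
; Overlapping an actor tagged Player casts it to BP_Player, calls TakeDamage and destroys the bullet.
; Actors tagged Enemy are ignored, while any other overlap destroys the bullet.
; An auto-destroy timer event removes the bullet after a short delay.
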(event Custom|Auto-destroy%20timer
  ;[1 1 1] Auto-destroy
  (Utilities|FlowControl|Delay 3.0)
  (Actor|DestroyActor))

(event Collision|EventActorBeginOverlap
  (params (OtherActor :type Actor%20Object%20Reference))
  ;[1 1 1] Collision
  (if (Actor|ActorHasTag OtherActor "Player")
    (bind _asbp_player (Utilities|Casting|CastToBP_Player OtherActor))
    (Default|TakeDamage _asbp_player)
    (Actor|DestroyActor)
    (elif (not (Actor|ActorHasTag OtherActor "Enemy"))
      (Actor|DestroyActor))))

(fn ConstructionScript)