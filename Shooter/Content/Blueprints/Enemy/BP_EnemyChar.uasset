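; Enemy character that chases and shoots the player, and dies when its HP runs out.
; Pawn sensing drives yaw-facing, AI movement and bullet spawning with sound and muzzle flash, throttled by a delay-based cooldown flag.
; TakeDamage lowers HP and triggers hit and death animations in the anim Blueprint, then on death fires the enemy-counter dispatcher and destroys the actor after a delay.
; Tick applies one-time damage if it falls below the world.
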(event OnSeePawn(PawnSensing)
  (params (Pawn :type Pawn%20Object%20Reference))
  (bind _scene (Variables|Default|GetScene))
  (bind _returnvalue (Transformation|GetWorldTransform _scene))
  ;[1 1 1] Follow and shoot player
  (bind _asbp_player (Utilities|Casting|CastToBP_Player Pawn))
  (if (> (Variables|Default|GetHP) 0)
    (Utilities|FlowControl|Sequence
      (:then_0
        (Transformation|SetActorRotation (Math|Rotator|MakeRotator 0.0 0.0 (.yaw (Math|Rotator|FindLookatRotation (Transformation|GetActorLocation) (Transformation|GetActorLocation _asbp_player)))))
        (AI|AIMoveTo self "0, 0, 0" _asbp_player 5.0 false))
      (:then_1
        (if (not (Variables|Default|GetShootCooldown))
          (bind _returnvalue_2 (Game|SpawnActorfromClass "/Game/Blueprints/Enemy/BP_Bullet.BP_Bullet_C" (Math|Transform|MakeTransform (.location _returnvalue) (.rotation _returnvalue) (Variables|Default|GetBulletScale)) "Undefined" 0 0))
          (Utilities|IsValid _returnvalue_2
            (:Is%20Valid
              (Default|Auto-destroyTimer _returnvalue_2)
              (Audio|PlaySoundatLocation "/Game/SFX/SC_EnemyShot.SC_EnemyShot" (.location _returnvalue) "0, 0, 0" 0.7 1.0 0.0 0 0 0 0)
              (Variables|Default|SetShootCooldown true)
              (bind _returnvalue_3 (Effects|SpawnEmitterAttached "/Game/InfinityBladeEffects/Effects/FX_Monsters/FX_Monster_Chicken/P_ChickenMaster_MuzzleFlash_01.P_ChickenMaster_MuzzleFlash_01" (Variables|Default|GetGunMuzzle) "None"))
              (Transformation|SetWorldScale3D _returnvalue_3 "0.500000,0.500000,0.500000")
              (Utilities|FlowControl|Delay 1.0)
              (Variables|Default|SetShootCooldown false))))))))

(event Custom|TakeDamage
  (params (Damage :type Integer))
  ;[1 1 1] Take damage
  (Variables|Default|SetHP (- (Variables|Default|GetHP) Damage))
  (bind _asue4asp_hero_tpp_anim_blueprint (Utilities|Casting|CastToUE4ASP_HeroTPP_AnimBlueprint (Components|SkeletalMesh|GetAnimInstance (Variables|Character|GetMesh))))
  (Default|TakeDamage _asue4asp_hero_tpp_anim_blueprint)
  ;[1 1 1] Die (if HP = 0)
  (if (<= (Variables|Default|GetHP) 0)
    (Default|Die _asue4asp_hero_tpp_anim_blueprint)
    (Default|CallEnemiesCounterUpdateD)
    (Utilities|FlowControl|Delay 2.0)
    (Actor|DestroyActor)))

(event EventTick
  (params (DeltaSeconds :type Float%20%28single-precision%29))
  (if (< (.z (Transformation|GetActorLocation)) -1e+03)
    (Utilities|FlowControl|DoOnce false
      (:Completed
        (CallFunction|TakeDamage 100)))))

(fn ConstructionScript)