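; BP_Rifle is a rifle pickup that attaches to the player's first-person mesh on overlap.
; Overlapping its sphere casts to BP_Player, sets HasGun, snaps the rifle to the GripPoint socket and binds to the player's ShootAnimD dispatcher.
; Its FireVFX event plays the first-person fire montage on that mesh and a laser sound at the rifle's location.
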(event OnComponentBeginOverlap(SphereCollision)
  (params (OverlappedComponent :type Primitive%20Component%20Object%20Reference) (OtherActor :type Actor%20Object%20Reference) (OtherComp :type Primitive%20Component%20Object%20Reference) (OtherBodyIndex :type Integer) (bFromSweep :type Boolean) (SweepResult :type Hit%20Result%20Structure%20%28by%20ref%29))
  ;[1 1 1] Weapon pick up
  (bind _asbp_player (Utilities|Casting|CastToBP_Player OtherActor))
  (Variables|Default|SetFirstPersonCharacterReference _asbp_player)
  (Variables|/Game/Blueprints/Player/BP_Player.BP_Player_C|SetHasGun _asbp_player true)
  (Transformation|AttachComponentToComponent self (Variables|/Game/Blueprints/Player/BP_Player.BP_Player_C|GetFirstPersonMesh (Variables|Default|GetFirstPersonCharacterReference)) "GripPoint" "SnapToTarget" "SnapToTarget" "SnapToTarget" true)
  (EventDispatchers|AssignShootAnimD (Variables|Default|GetFirstPersonCharacterReference) (EventDispatchers|CreateEvent :!event Custom|FireVFX)))

(event Custom|FireVFX
  ;[1 1 1] Fire VFX
  (Animation|Montage|MontagePlay (Components|SkeletalMesh|GetAnimInstance (Variables|/Game/Blueprints/Player/BP_Player.BP_Player_C|GetFirstPersonMesh (Variables|Default|GetFirstPersonCharacterReference))) "/Game/FirstPersonArms/Animations/FirstPersonFire_Montage.FirstPersonFire_Montage" 1.0 "MontageLength" 0.0 true)
  (Audio|PlaySoundatLocation "/Game/SFX/SC_Laser.SC_Laser" (Transformation|GetActorLocation) "0, 0, 0" 1.0 1.0 0.0 0 0 0 0))

(fn ConstructionScript)